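; BP_pickable is a physics-simulated ammo item that carries bullet info: damage, color, material and mesh.
; On BeginPlay its static mesh becomes movable and starts simulating physics.
; SetData stores that info, swaps the mesh, and tints the supplied dynamic material through its "color" parameter before applying it.
; GetData packs the current values back into a bullet info struct.
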(event `self.ReceiveBeginPlay`
  (bind _staticmesh (`self.StaticMesh`))
  (`SceneComponent.SetMobility` _staticmesh "Movable")
  (`PrimitiveComponent.SetSimulatePhysics` _staticmesh true))

(event `/Game/blueprints/BPI/BPI_Ammo.SetData`
  (params (data :type "/Game/blueprints/BPI/BulletData Structure"))
  (bind (_x _y _z) (`KismetMathLibrary.BreakVector3f` data_Color_7_A7172CCC480B950AF58FA68A552E7E10))
  (set `self.Damages` data_Damages_2_DB97FBFE448D7D847B2EF699AE72A2F5)
  (bind _output_get (set `self.DynamicMat` data_Material_17_4BD1951A439DA13E5FD9748A5B1F3ADA))
  (`StaticMeshComponent.SetStaticMesh` (`self.StaticMesh`) data_SM_18_97A56FA3440EA60E96E74681C242ED14)
  (set `self.color` data_Color_7_A7172CCC480B950AF58FA68A552E7E10)
  (`MaterialInstanceDynamic.SetVectorParameterValue` _output_get "color" (make `LinearColor` _x _y _z 1.0))
  (`PrimitiveComponent.SetMaterial` (`self.StaticMesh`) 0 (`self.DynamicMat`)))

(fn `GetData`
  (returns (GetbulletInfo :type "/Game/blueprints/BPI/BulletData Structure"))
  (return (make `/Game/blueprints/BPI/BulletData` (`self.Damages`) (`self.color`) (`self.DynamicMat`) (`StaticMeshComponent.StaticMesh` (`self.StaticMesh`)))))

(fn `UserConstructionScript`)